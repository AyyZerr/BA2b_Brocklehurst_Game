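; A plant actor whose health drains over time and is shown on a Plant_Healthbar widget.
; Tick deals periodic damage to itself, and AnyDamage clamps Health and updates HealthPercent.
; BeginPlay fills health and hands the plant reference to its widget component's healthbar.
; Box overlaps track whether the ThirdPersonCharacter is near in PlayerInRange, which these graphs set but never read.
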(event OnComponentBeginOverlap(Box)
  (params (OverlappedComponent :type Primitive%20Component%20Object%20Reference) (OtherActor :type Actor%20Object%20Reference) (OtherComp :type Primitive%20Component%20Object%20Reference) (OtherBodyIndex :type Integer) (bFromSweep :type Boolean) (SweepResult :type Hit%20Result%20Structure%20%28by%20ref%29))
  (Utilities|Casting|CastToThirdPersonCharacter OtherActor)
  (Variables|Default|SetPlayer_In_Range true))

(event OnComponentEndOverlap(Box)
  (params (OverlappedComponent :type Primitive%20Component%20Object%20Reference) (OtherActor :type Actor%20Object%20Reference) (OtherComp :type Primitive%20Component%20Object%20Reference) (OtherBodyIndex :type Integer))
  (Utilities|Casting|CastToThirdPersonCharacter OtherActor)
  (Variables|Default|SetPlayer_In_Range false))

(event Game|Damage|EventAnyDamage
  (params (Damage :type Float%20%28single-precision%29) (DamageType :type Damage%20Type%20Object%20Reference) (InstigatedBy :type Controller%20Object%20Reference) (DamageCauser :type Actor%20Object%20Reference))
  (Variables|Default|SetHealth (Math|Float|Clamp(Float) (- (Variables|Default|GetHealth) Damage) 0.0 (Variables|Default|GetMax_Health)))
  (Variables|Default|SetHealth_Percent (/ (Variables|Default|GetHealth) (Variables|Default|GetMax_Health))))

(event EventBeginPlay
  (Variables|Default|SetHealth (Variables|Default|GetMax_Health))
  (bind _asplant_healthbar (Utilities|Casting|CastToPlant_Healthbar (UserInterface|GetUserWidgetObject (Variables|Default|GetWidget))))
  (Variables|/Game/Blueprints/Plant_Healthbar.Plant_Healthbar_C|SetPlant _asplant_healthbar self))

(event EventTick
  (params (DeltaSeconds :type Float%20%28single-precision%29))
  (bind _output_get (Variables|Default|SetTime (+ (Variables|Default|GetTime) DeltaSeconds)))
  (if (>= _output_get 3.0)
    (Variables|Default|SetTime 0.0)
    (Game|Damage|ApplyDamage self 1e+01 0 0)))

(fn ConstructionScript)